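; EvilCubePawn is an enemy cube pawn that starts with two health and destroys any actor that hits its Cube component.
; Each hit costs one health and spawns an explosion effect at the cube, with the final hit also destroying the Cube component.
; An end-play event on FireExplosion destroys the pawn.
; A separate Hurt function decrements health and destroys the pawn immediately when it runs out.
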(event `self.Cube.OnComponentHit`
  (params (HitComponent :type "PrimitiveComponent Object Reference") (OtherActor :type "Actor Object Reference") (OtherComp :type "PrimitiveComponent Object Reference") (NormalImpulse :type "Vector Structure") (Hit :type "HitResult Structure (by ref)"))
  (bind _health (`self.Health`))
  (`self.K2_DestroyActor` OtherActor)
  (`/Engine/EditorBlueprintResources/StandardMacros.DecrementInt` _health
    (:`  `
      (if (> _health 0)
        (bind _returnvalue (`|SpawnActorFromClass` "/Game/StarterContent/Blueprints/Blueprint_Effect_Explosion.Blueprint_Effect_Explosion_C" (`SceneComponent.K2_GetComponentToWorld` (`self.Cube`)) "Undefined" "OverrideRootScale" null null :!label _label))
        (set `self.FireExplosion` _returnvalue)
        (else
          (`|ExecutionSequence`
            (:`then_0`
              (goto _label))
            (:`then_1`
              (`ActorComponent.K2_DestroyComponent` (`self.Cube`)))))))))

(event `self.FireExplosion.OnEndPlay`
  (params (Actor :type "Actor Object Reference") (EndPlayReason :type "EEndPlayReason Enum" :default "Destroyed"))
  (`self.K2_DestroyActor`))

(event `self.ReceiveBeginPlay`
  (set `self.Health` 2))

(fn `Hurt`
  (bind _result (`/Engine/EditorBlueprintResources/StandardMacros.DecrementInt` (`self.Health`))
    (:`  `
      (if (> _result 0)
        (return)
        (else
          (`self.K2_DestroyActor`)
          (return))))))

(fn `UserConstructionScript`)