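; Proximity interaction for a crow: pressing Interact in range spawns an actor at the parent actor's transform and destroys the parent.
; Tick compares the parent's distance to the player character against a fixed radius, toggling a display flag and the Interaction_E_Template prompt widget.
; The flag gates the Interact input.
; Prompt removal looks up top-level widgets by class instead of keeping a reference to the created widget.
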(event `InputAction|Interact` :consume false :overrideparent false
  (params (Key :type "Key Structure"))
  (bind _returnvalue (`self.GetParentActor`))
  (:`Pressed`
    (if (`self.IsDisplayingInteraction`)
      (`|SpawnActorFromClass` "/Game/StarterContent/Blueprints/Blueprint_Effect_Explosion.Blueprint_Effect_Explosion_C" (`self.GetTransform` _returnvalue) "Undefined" "OverrideRootScale" null null)
      (`self.K2_DestroyActor` _returnvalue)
      (bind _foundwidgets (`WidgetBlueprintLibrary.GetAllWidgetsOfClass` "/Game/Blueprints/Interaction_E_Template.Interaction_E_Template_C"))
      (`Widget.RemoveFromParent` _foundwidgets))))

(event `self.ReceiveBeginPlay`
  (set `self.IsDisplayingInteraction` false))

(event `self.ReceiveTick`
  (params (DeltaSeconds :type "Float (single-precision)"))
  (if (<= (`KismetMathLibrary.Vector_Distance` (`self.K2_GetActorLocation` (`self.GetParentActor`)) (`self.K2_GetActorLocation` (`GameplayStatics.GetPlayerCharacter` 0))) 200.0)
    (if (not (`self.IsDisplayingInteraction`))
      (set `self.IsDisplayingInteraction` true)
      (bind _returnvalue (`|CreateWidget` "/Game/Blueprints/Interaction_E_Template.Interaction_E_Template_C"))
      (`UserWidget.AddToViewport` _returnvalue 0))
    (elif (`self.IsDisplayingInteraction`)
      (set `self.IsDisplayingInteraction` false)
      (bind _foundwidgets (`WidgetBlueprintLibrary.GetAllWidgetsOfClass` "/Game/Blueprints/Interaction_E_Template.Interaction_E_Template_C"))
      (`Widget.RemoveFromParent` _foundwidgets))))

(fn `UserConstructionScript`)