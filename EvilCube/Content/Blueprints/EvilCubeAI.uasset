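; EvilCubeAI is AI controller logic that makes its controlled pawn follow the player character.
; A looping timer started on BeginPlay runs FollowPlayer every 0.1 seconds to check the horizontal distance between pawn and player.
; Beyond a fixed range it issues AI Move To toward the player; otherwise it targets the pawn itself, in effect halting the chase.
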(event `self.ReceiveBeginPlay`
  (`KismetSystemLibrary.K2_SetTimer` null "FollowPlayer" 0.1 true))

(event `FollowPlayer`
  (bind _returnvalue (`GameplayStatics.GetPlayerCharacter` 0))
  (bind _returnvalue_2 (`self.K2_GetPawn`))
  (bind _returnvalue_3 (`self.K2_GetActorLocation` _returnvalue_2))
  (if (> (`KismetMathLibrary.Distance2D` (`KismetMathLibrary.Conv_VectorToVector2D` _returnvalue_3) (`KismetMathLibrary.Conv_VectorToVector2D` (`self.K2_GetActorLocation` _returnvalue))) 600.0)
    (`|AIMoveTo` null (0.0 0.0 0.0) _returnvalue)
    (else
      (`|AIMoveTo` null _returnvalue_3 _returnvalue_2))))

(event `self.ReceiveTick`
  (params (DeltaSeconds :type "Float (single-precision)")))

(fn `UserConstructionScript`)