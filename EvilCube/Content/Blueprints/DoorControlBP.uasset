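; Proximity door actor that slides up when the player pawn comes within a horizontal open distance and lowers otherwise, unless locked.
; BeginPlay turns the travel distance into an absolute upper Z limit and copies it to the variable behind the lower limit, which adds a hardcoded offset.
; Tick moves the door by a fixed, frame-rate-dependent step without sweeping.
; CurZ is written but never read, and receives Y values during movement.
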(event `self.ReceiveBeginPlay`
  (bind _z (.z (`self.K2_GetActorLocation`)))
  (set `self.CurZ` _z)
  (bind _output_get (set `self.DistanceZ` (+ _z (`self.DistanceZ`))))
  (bind _output_get_2 (set `self.DistanceZNeg` _output_get))
  (`/Engine/EditorBlueprintResources/StandardMacros.NegateFloat` _output_get_2))

(event `self.ReceiveTick`
  (params (DeltaSeconds :type "Float (single-precision)"))
  (bind _returnvalue (`self.K2_GetActorLocation`))
  (bind _z (.z (`self.K2_GetActorLocation`)))
  (bind _returnvalue_2 (+ _returnvalue (0.0 0.0 2.0)))
  (bind _returnvalue_3 (+ _returnvalue (0.0 0.0 -2.0)))
  (if (`self.Locked`)
    _
    (elif (<= (`KismetMathLibrary.Vector_Distance2D` (`self.K2_GetActorLocation` (`GameplayStatics.GetPlayerPawn` 0)) _returnvalue) (`self.OpenDistance`))
      (if (< _z (`self.DistanceZ`))
        (`self.K2_SetActorLocation` _returnvalue_2)
        (set `self.CurZ` (.y _returnvalue_3)))
      (elif (not (< _z (+ (`self.DistanceZNeg`) 120.0)))
        (`self.K2_SetActorLocation` _returnvalue_3)
        (set `self.CurZ` (.y _returnvalue_2))))))

(fn `UserConstructionScript`)