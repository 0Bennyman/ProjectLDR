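; Buildable turret actor that turns toward the nearest EvilCubePawn within range.
; Tick scans all EvilCubePawns by distance and eases the actor's rotation toward a point slightly below the closest one.
; A looping timer runs RaycastForward, a debug-drawn forward line trace from Cube1 whose result is unused.
; ShootBall spawns a FirstPersonProjectile at ShootPoint when a target is in range, but nothing here calls it.
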(event `self.ReceiveBeginPlay`
  (`KismetSystemLibrary.K2_SetTimer` self "RaycastForward" 0.1 true))

(event `self.ReceiveTick`
  (params (DeltaSeconds :type "Float (single-precision)"))
  (set `self.lowestDistance` 800.0)
  (`|ExecutionSequence`
    (:`then_0`
      (bind _outactors (`GameplayStatics.GetAllActorsOfClass` "/Game/Blueprints/EvilCubePawn.EvilCubePawn_C"))
      (for _array_element _outactors
        (bind _returnvalue (`self.GetDistanceTo` _array_element self))
        (if (< _returnvalue (`self.lowestDistance`))
          (set `self.lowestDistance` _returnvalue)
          (set `self.ClosestPawn` _array_element))))
    (:`then_1`
      (if (< (`self.lowestDistance`) 800.0)
        (`self.K2_SetActorRotation` (`KismetMathLibrary.RInterpTo` (`SceneComponent.K2_GetComponentRotation` (`self.DefaultSceneRoot`)) (`KismetMathLibrary.FindLookAtRotation` (`self.K2_GetActorLocation`) (+ (`self.K2_GetActorLocation` (`self.ClosestPawn`)) (0.0 0.0 -50.0))) 0.5 0.05))))))

(fn `RaycastForward`
  (bind _returnvalue (`SceneComponent.K2_GetComponentLocation` (`self.Cube1`)))
  (bind _returnvalue_2 (`SceneComponent.K2_GetComponentRotation` (`self.DefaultSceneRoot`)))
  (`KismetSystemLibrary.LineTraceSingle` :`Start` _returnvalue :`End` (`KismetMathLibrary.TransformLocation` (`KismetMathLibrary.MakeTransform` (+ _returnvalue (`KismetMathLibrary.GreaterGreater_VectorRotator` (100.0 0.0 -10.0) _returnvalue_2)) _returnvalue_2) (5000.0 50.0 -180.0)) :`TraceChannel` "TraceTypeQuery1" :`bTraceComplex` true :`DrawDebugType` "ForDuration" :`DrawTime` 1.0)
  (return))

(fn `ShootBall`
  (if (< (`self.lowestDistance`) 800.0)
    (`|SpawnActorFromClass` "/Game/FirstPersonBP/Blueprints/FirstPersonProjectile.FirstPersonProjectile_C" (`KismetMathLibrary.Conv_VectorToTransform` (`SceneComponent.K2_GetComponentLocation` (`self.ShootPoint`))) "Undefined" "OverrideRootScale" null null)
    (return)
    (else
      (return))))

(fn `UserConstructionScript`)